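; DB is an Actor Blueprint whose AplicarOpcionesGraficos function applies graphics options stored in a Preferences array.
; It builds an r.setres console command from the stored width, height and windowed or fullscreen flag.
; It then maps stored levels to view distance and anti-aliasing commands, and appends the remaining values to post-process, shadow, texture and effects scalability commands.
; The event graph and construction script are empty.
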(fn `AplicarOpcionesGraficos`
  (locals (resolutionString :type String) (visionString :type String))
  (bind _preferences (`self.Preferences`))
  (bind _returnvalue (`KismetStringLibrary.Concat_StrStr` "r.setres " (`KismetStringLibrary.Concat_StrStr` (`|GetArrayItem` _preferences) "x" (`|GetArrayItem` _preferences 1))))
  (if (`KismetStringLibrary.EqualEqual_StrStr` (`|GetArrayItem` _preferences 2) "0")
    (set `local.resolutionString` (`KismetStringLibrary.Concat_StrStr` _returnvalue "w"))
    (else
      (set `local.resolutionString` (`KismetStringLibrary.Concat_StrStr` _returnvalue "f"))))
  (`KismetSystemLibrary.ExecuteConsoleCommand` (`local.resolutionString`))
  (switch `string` (`|GetArrayItem` _preferences 4)
    (:`0`
      (`KismetSystemLibrary.ExecuteConsoleCommand` "r.ViewDistanceScale 0.4"))
    (:`1`
      (`KismetSystemLibrary.ExecuteConsoleCommand` "r.ViewDistanceScale 0.7"))
    (:`2`
      (`KismetSystemLibrary.ExecuteConsoleCommand` "r.ViewDistanceScale 1.0")))
  (switch `string` (`|GetArrayItem` _preferences 5)
    (:`0`
      (`KismetSystemLibrary.ExecuteConsoleCommand` "r.PostProcessAAQuality 0"))
    (:`1`
      (`KismetSystemLibrary.ExecuteConsoleCommand` "r.PostProcessAAQuality 2"))
    (:`2`
      (`KismetSystemLibrary.ExecuteConsoleCommand` "r.PostProcessAAQuality 4"))
    (:`3`
      (`KismetSystemLibrary.ExecuteConsoleCommand` "r.PostProcessAAQuality 6")))
  (`KismetSystemLibrary.ExecuteConsoleCommand` (`KismetStringLibrary.Concat_StrStr` "sg.PostProcessQuality " (`|GetArrayItem` _preferences 6)))
  (`KismetSystemLibrary.ExecuteConsoleCommand` (`KismetStringLibrary.Concat_StrStr` "sg.ShadowQuality " (`|GetArrayItem` _preferences 7)))
  (`KismetSystemLibrary.ExecuteConsoleCommand` (`KismetStringLibrary.Concat_StrStr` "sg.TextureQuality " (`|GetArrayItem` _preferences 8)))
  (`KismetSystemLibrary.ExecuteConsoleCommand` (`KismetStringLibrary.Concat_StrStr` "sg.EffectsQuality " (`|GetArrayItem` _preferences 9))))

(fn `UserConstructionScript`)